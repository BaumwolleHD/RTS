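; Default game mode that registers each joining player in the DefaultGamestate on login.
; On PostLogin it waits a zero-length delay, then on the authority adds the player's PlayerState and controlled pawn to the gamestate's player lists.
; The index returned from the PlayerState list is stored as CurrentUserIndex on that player's DefaultPlayerstate.
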(event `self.ReceiveTick`
  (params (DeltaSeconds :type "Float (single-precision)")))

(event `self.K2_PostLogin`
  (params (NewPlayer :type "PlayerController Object Reference"))
  (bind _playerstate (`Controller.PlayerState` NewPlayer))
  (bind _asdefault_gamestate (cast `DefaultGamestate` (`GameplayStatics.GetGameState`) :!pure true))
  (`KismetSystemLibrary.Delay` 0.0)
  (`/Engine/EditorBlueprintResources/ActorMacros.Switch Has Authority`
    (:`Authority`
      (bind _returnvalue (`KismetArrayLibrary.Array_Add` (`DefaultGamestate.PlayerStateList` _asdefault_gamestate) _playerstate))
      (`KismetArrayLibrary.Array_Add` (`DefaultGamestate.PlayerCharacterList` _asdefault_gamestate) (`Controller.K2_GetPawn` NewPlayer))
      (bind _asdefault_playerstate (cast `DefaultPlayerstate` _playerstate))
      (set `DefaultPlayerstate.CurrentUserIndex` _returnvalue _asdefault_playerstate))))

(fn `UserConstructionScript`)