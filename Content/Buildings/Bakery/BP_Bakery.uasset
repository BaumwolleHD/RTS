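; Bakery building Blueprint that shows fire and smoke effects while its growing phase is active.
; GrowingStarted activates the smoke, opens a gate and plays a timeline that drives the fire light's intensity.
; The timeline replays on finish through that gate, looping until GrowingComplete stops it, closes the gate, zeroes the light and deactivates the smoke.
; BuildingComplete is an empty event.
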(event `self.ReceiveBeginPlay`)

(event `self.ReceiveActorBeginOverlap`
  (params (OtherActor :type "Actor Object Reference")))

(event `self.ReceiveTick`
  (params (DeltaSeconds :type "Float (single-precision)")))

(event `self.BuildingComplete`)

(event `self.GrowingComplete`
  (bind _smoke (`self.Smoke`))
  (`LightComponent.SetIntensity` (`self.FireLight`) 0.0)
  (`SceneComponent.SetHiddenInGame` _smoke false false)
  (`ActorComponent.Deactivate` _smoke)
  (`|ExecutionSequence`
    (:`then_0`
      (bind (_direction _brightness) (`Timeline|FireTimeline` :!via `Stop` :!label _label)
        (:`Update`
          (`LightComponent.SetIntensity` (`self.FireLight`) (* _brightness 100.0)))
        (:`Finished`
          (`/Engine/EditorBlueprintResources/StandardMacros.Gate` true :!label _label_2
            (:`Exit`
              (goto _label :!via `PlayFromStart`))))))
    (:`then_1`
      (goto _label_2 :!via `Close`))))

(event `self.GrowingStarted`
  (bind _smoke (`self.Smoke`))
  (`SceneComponent.SetHiddenInGame` _smoke false false)
  (`ActorComponent.Activate` _smoke true)
  (`|ExecutionSequence`
    (:`then_0`
      (goto _label_2 :!via `Open`))
    (:`then_1`
      (goto _label))))

(fn `UserConstructionScript`)