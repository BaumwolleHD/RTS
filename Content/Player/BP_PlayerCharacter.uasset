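; BP_PlayerCharacter is the player character, holding the selected building class, a Mode state and lists of owned NPCs.
; On non-authority instances, BeginPlay uses timed delays to switch the selection from farm to storage block, print its class name and set Mode to Idle.
; An unconnected chain would spawn a scaled NPC, register it as a storage worker via its controller, then join that sequence.
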(event `self.ReceiveBeginPlay`
  (`/Engine/EditorBlueprintResources/ActorMacros.Switch Has Authority`
    (:`Remote`
      (`KismetSystemLibrary.Delay` 2.0)
      (set `self.SelectedBuilding` "/Game/Buildings/Farm/BP_Farm.BP_Farm_C")
      (`KismetSystemLibrary.Delay` 2.0)
      (bind _output_get (set `self.SelectedBuilding` "/Game/Buildings/StorageBlock/BP_StorageBlock.BP_StorageBlock_C"))
      (`KismetSystemLibrary.Delay` 2.0)
      (`KismetSystemLibrary.PrintString` (`KismetSystemLibrary.GetClassDisplayName` _output_get))
      (set `self.Mode` "Idle"))))

(event `self.ReceiveActorBeginOverlap`
  (params (OtherActor :type "Actor Object Reference")))

(fn `UserConstructionScript`)